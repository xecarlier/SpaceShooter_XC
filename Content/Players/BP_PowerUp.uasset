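; BP_PowerUp is a pickup actor that becomes one of three power-up types at random: attack rate, invincibility or life.
; On BeginPlay it stores the chosen type in PowerUpType and tints its sphere through a dynamic material instance, with a different color per type.
; UsePowerUp spawns a spark effect and plays a sound, then after a short delay removes the emitter and destroys the actor.
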(event Custom|UsePowerUp
  (bind _returnvalue (Effects|SpawnEmitteratLocation "/Game/StarterContent/Particles/P_Sparks.P_Sparks" (Transformation|GetActorLocation)))
  (Audio|PlaySound2D "/Game/Players/powerUp.powerUp" 1.0 1.0 0.0 0 0)
  (Utilities|FlowControl|Delay 0.4)
  (Components|DestroyComponent _returnvalue)
  (Actor|DestroyActor))

(event EventBeginPlay
  (bind _output_get (Variables|Default|SetRandInt (Math|Random|RandomInteger 3)))
  (if (== _output_get 0)
    (Variables|Default|SetPowerUpType "AtkRate")
    (bind _returnvalue (Rendering|Material|CreateDynamicMaterialInstance (Variables|Default|GetSphere) 0 "/Game/Players/M_Power_Up.M_Power_Up" "None" :!class /Script/Engine.PrimitiveComponent))
    (Rendering|Material|SetVectorParameterValue _returnvalue "SunColor" "(R=1.000000,G=0.031026,B=0.050922,A=1.000000)" :!class /Script/Engine.MaterialInstanceDynamic)
    (elif (== _output_get 1)
      (Variables|Default|SetPowerUpType "Invincibility")
      (bind _returnvalue_2 (Rendering|Material|CreateDynamicMaterialInstance (Variables|Default|GetSphere) 0 "/Game/Players/M_Power_Up.M_Power_Up" "None" :!class /Script/Engine.PrimitiveComponent))
      (Rendering|Material|SetVectorParameterValue _returnvalue_2 "SunColor" "(R=0.422844,G=0.085170,B=1.000000,A=1.000000)" :!class /Script/Engine.MaterialInstanceDynamic)
      (elif (== _output_get 2)
        (Variables|Default|SetPowerUpType "Life")
        (bind _returnvalue_3 (Rendering|Material|CreateDynamicMaterialInstance (Variables|Default|GetSphere) 0 "/Game/Players/M_Power_Up.M_Power_Up" "None" :!class /Script/Engine.PrimitiveComponent))
        (Rendering|Material|SetVectorParameterValue _returnvalue_3 "SunColor" "(R=0.116546,G=1.000000,B=0.231627,A=1.000000)" :!class /Script/Engine.MaterialInstanceDynamic)))))

(fn ConstructionScript)